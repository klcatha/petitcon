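; Player controller for a lap-based racing game, managing race flow, HUD, best-time records and vehicle respawning.
; A left click runs the countdown, then starts race and lap timelines that track times and hide missed gold, silver and bronze goals.
; Lap updates save record lap and race times to a SaveGame slot and play HUD animations.
; R resets records before the race, and Restart reloads the level after a delay.
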(event `self.ReceiveBeginPlay`
  ;[1 1 1] Event Begin Play / Get Reference
  (bind _returnvalue (`|CreateWidget` "/Game/Blueprints/UI/HUD.HUD_C"))
  (bind _output_get (set `self.HUDReference` _returnvalue))
  (`UserWidget.AddToViewport` _output_get 0)
  (bind _asvehicle_blueprint (cast `/Game/VehicleAdvBP/Blueprints/VehicleBlueprint` (`GameplayStatics.GetPlayerPawn` 0)))
  (set `self.VehicleReference` _asvehicle_blueprint))

(event `StartGameSetup`
  ;[1 1 1] ゲームシーケンスの開始とセーブファイルを確認してテキストの初期化
  (`self.SaveGameCheck`)
  (`self.InitText`))

(event `StartRaceTime`
  ;[1 1 1] レース全体の進行時間をテキスト形式に変換して表示
  (bind (_direction _time) (`Timeline|GameTime` :!label _label)
    (:`Update`
      (bind _output_get (set `self.ActualRaceTime` _time))
      (set `self.RaceTimeText` (`/Game/Blueprints/TimeConversion.TimeToText` _output_get))
      (`self.UpdateGoals`))))

(event `Restart`
  ;[1 1 1] レースが終わったらマップを再読み込み
  (set `self.RaceStart` false)
  (`KismetSystemLibrary.Delay` 6.0)
  (`KismetSystemLibrary.ExecuteConsoleCommand` "RestartLevel"))

(event `StopRaceTime`
  ;[1 1 1] レース全体の進行時間をテキスト形式に変換して表示
  (goto _label :!via `Stop`))

(event `StartLapTime`
  ;[1 1 1] レース全体の進行時間をテキスト形式に変換して表示
  (bind (_direction _time) (`Timeline|LapTime` :!via `PlayFromStart` :!label _label_2)
    (:`Update`
      (set `self.ActualLapTime` _time))))

(event `UpdateLap`
  ;[1 1 1] ラップ数を更新、ラップタイムを更新するかどうか
  (if (not (`self.RaceComplete`))
    (bind _output_get (set `self.ActualLap` (+ (`self.ActualLap`) 1)))
    (set `self.CurrentLapText` (`KismetTextLibrary.Conv_IntToText` _output_get)))
  (`self.LapTimeCheck`))

(event `StopLapTime`
  ;[1 1 1] レース全体の進行時間をテキスト形式に変換して表示
  (goto _label_2 :!via `Stop`))

(event `Key|R`
  (params (Key :type "Key Structure" :default "AnyKey"))
  ;[1 1 1] レースが開始されていない場合デフォルトの記録を設定する
  (:`Pressed`
    (if (not (`self.RaceStart`))
      (set `self.BestLapTime` (`self.DefaultBestLapTime`))
      (set `self.BestRaceTime` (`self.DefaultBestRaceTime`))
      (`self.SaveTheGame`)
      (`self.InitText`))))

(event `RespawnVehicle`
  ;[1 1 1] スポーン
  (bind _returnvalue (`|SpawnActorFromClass` "/Game/VehicleAdvBP/Blueprints/VehicleBlueprint.VehicleBlueprint_C" (`self.RespawnLocation`) "Undefined" "OverrideRootScale"))
  (`self.Possess` _returnvalue))

(event `Key|LeftMouseButton`
  (params (Key :type "Key Structure" :default "AnyKey"))
  (bind _hudreference (`self.HUDReference`))
  (bind _hudreference_2 (`self.HUDReference`))
  ;[1 1 1] マウスの左クリックでレース開始
  (:`Pressed`
    (`/Engine/EditorBlueprintResources/StandardMacros.DoOnce` false
      (:`Completed`
        (set `/Game/Blueprints/UI/HUD.SplashScreenVisible` "Hidden" _hudreference)
        (set `/Game/Blueprints/UI/HUD.CountdownVisible` "Visible" _hudreference)
        (`UserWidget.PlayAnimation` _hudreference (`/Game/Blueprints/UI/HUD.CountdownAnimation` _hudreference) 0.0 1 "Forward" 1.0)
        (`KismetSystemLibrary.Delay` 2.5)
        (set `self.ReadyText` "3")
        (`KismetSystemLibrary.Delay` 1.0)
        (set `self.ReadyText` "2")
        (`KismetSystemLibrary.Delay` 1.0)
        (set `self.ReadyText` "1")
        (`KismetSystemLibrary.Delay` 1.0)
        (set `self.ReadyText` "GO!")
        (`KismetSystemLibrary.Delay` 1.0)
        (set `/Game/Blueprints/UI/HUD.CountdownVisible` "Hidden" _hudreference_2)
        (set `/Game/Blueprints/UI/HUD.GameHUDVisible` "Visible" _hudreference_2)
        (set `self.RaceStart` true)
        (`self.StartRaceTime`)
        (`self.StartLapTime`)))))

(fn `InitText`
  ;[1 1 1] ラップ数とタイムを変換してテキストにセット
  (set `self.CurrentLapText` (`KismetTextLibrary.Conv_IntToText` (`self.ActualLap`)))
  (set `self.MaxLapText` (`KismetTextLibrary.Conv_IntToText` (`self.MaxLaps`)))
  (set `self.GoldTimeText` (`/Game/Blueprints/TimeConversion.TimeToText` (`self.GoldTime`)))
  (set `self.SilverTimeText` (`/Game/Blueprints/TimeConversion.TimeToText` (`self.SilverTime`)))
  (set `self.BronzeTimeText` (`/Game/Blueprints/TimeConversion.TimeToText` (`self.BronzeTime`)))
  (set `self.BestLapText` (`/Game/Blueprints/TimeConversion.TimeToText` (`self.BestLapTime`)))
  (set `self.BestTimeText` (`/Game/Blueprints/TimeConversion.TimeToText` (`self.BestRaceTime`))))

(fn `LapTimeCheck`
  (bind _hudreference (`self.HUDReference`))
  ;[1 1 1] ラップタイムを確認してタイムレコードを樹立した場合保存する
  (`self.StopLapTime`)
  (if (<= (`self.ActualLapTime`) (`self.BestLapTime`))
    (bind _output_get (set `self.BestLapTime` (`self.ActualLapTime`)))
    (set `self.BestLapText` (`/Game/Blueprints/TimeConversion.TimeToText` _output_get))
    (`self.SaveTheGame`)
    (`UserWidget.PlayAnimation` _hudreference (`/Game/Blueprints/UI/HUD.LapRecordAnimation` _hudreference) 0.0 1 "Forward" 1.0)
    (set `self.ActualLapTime` 0.0)
    (else
      (set `self.ActualLapTime` 0.0)))
  (if (`self.RaceComplete`)
    (`self.RaceTimeCheck`)
    (else
      (`self.StartLapTime`))))

(fn `LoadTheGame`
  ;[1 1 1] ベストのラップタイムとレースタイムを読み込む
  (bind _returnvalue (`GameplayStatics.LoadGameFromSlot` (`self.SaveSlot`)))
  (bind _asmy_save_game (cast `/Game/Blueprints/MySaveGame` _returnvalue))
  (set `self.BestLapTime` (`/Game/Blueprints/MySaveGame.SavedBestLap` _asmy_save_game))
  (set `self.BestRaceTime` (`/Game/Blueprints/MySaveGame.SavedBestTime` _asmy_save_game)))

(fn `RaceTimeCheck`
  (bind _hudreference (`self.HUDReference`))
  ;[1 1 1] レースタイムを確認し、新記録を樹立していた場合はほぞんする
  (`self.StopRaceTime`)
  (if (<= (`self.ActualRaceTime`) (`self.BestRaceTime`))
    (bind _output_get (set `self.BestRaceTime` (`self.ActualRaceTime`)))
    (set `self.BestTimeText` (`/Game/Blueprints/TimeConversion.TimeToText` _output_get))
    (`self.SaveTheGame`)
    (`UserWidget.PlayAnimation` _hudreference (`/Game/Blueprints/UI/HUD.RaceRecordAnimation` _hudreference) 0.0 1 "Forward" 1.0)))

(fn `SaveGameCheck`
  ;[1 1 1] 既存のセーブデータがあるかを確認、もし存在するならロード、なければ記録を上書きしてセーブ
  (bind _returnvalue (`GameplayStatics.DoesSaveGameExist` (`self.SaveSlot`)))
  (if _returnvalue
    (`self.LoadTheGame`)
    (else
      (set `self.BestLapTime` (`self.DefaultBestLapTime`))
      (set `self.BestRaceTime` (`self.DefaultBestRaceTime`))
      (`self.SaveTheGame`))))

(fn `SaveTheGame`
  ;[1 1 1] スロットにラップタイムとレースタイムをセーブする
  (bind _returnvalue (`GameplayStatics.CreateSaveGameObject` "/Game/Blueprints/MySaveGame.MySaveGame_C"))
  (bind _output_get (set `self.SaveGameReference` _returnvalue))
  (bind _asmy_save_game (cast `/Game/Blueprints/MySaveGame` _output_get))
  (set `/Game/Blueprints/MySaveGame.SavedBestLap` (`self.BestLapTime`) _asmy_save_game)
  (set `/Game/Blueprints/MySaveGame.SavedBestTime` (`self.BestRaceTime`) _asmy_save_game)
  (`GameplayStatics.SaveGameToSlot` (`self.SaveGameReference`) (`self.SaveSlot`)))

(fn `UpdateGoals`
  ;[1 1 1] 目標時間を達成できない場合は該当するHUDを隠す
  (if (not (<= (`self.ActualRaceTime`) (`self.GoldTime`)))
    (`|ExecutionSequence`
      (:`then_0`
        (`/Engine/EditorBlueprintResources/StandardMacros.DoOnce` false
          (:`Completed`
            (set `/Game/Blueprints/UI/HUD.GoldTimeVisible` "Hidden" (`self.HUDReference`)))))
      (:`then_1`
        (if (not (<= (`self.ActualRaceTime`) (`self.SilverTime`)))
          (`|ExecutionSequence`
            (:`then_0`
              (`/Engine/EditorBlueprintResources/StandardMacros.DoOnce` false
                (:`Completed`
                  (set `/Game/Blueprints/UI/HUD.SilverTimeVisible` "Hidden" (`self.HUDReference`)))))
            (:`then_1`
              (if (not (<= (`self.ActualRaceTime`) (`self.BronzeTime`)))
                (`/Engine/EditorBlueprintResources/StandardMacros.DoOnce` false
                  (:`Completed`
                    (set `/Game/Blueprints/UI/HUD.BronzeTimeVisible` "Hidden" (`self.HUDReference`))))))))))))

(fn `UserConstructionScript`)