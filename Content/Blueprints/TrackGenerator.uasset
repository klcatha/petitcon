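; TrackGenerator is a Blueprint that builds a looping road track along a spline in its construction script.
; It stores the spline point count, then grows or trims RoadDataArray to match it, though the mesh build does not read that array.
; For each point it adds a spline mesh component using RoadMesh, fitted to the local locations and tangents of that point and the next, wrapping last to first.
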(fn `Build Track Element`
  (params (LoopIndex :type Integer) (TrackElementMesh :type "StaticMesh Object Reference"))
  (locals (LocaL_CurrentLoopIndex :type Integer) (LocaL_NextLoopIndex :type Integer) (LocaL_TrackElementMesh :type "StaticMesh Object Reference") (LocaL_StartLocation :type "Vector Structure") (LocaL_StartTangent :type "Vector Structure") (LocaL_EndLocation :type "Vector Structure") (LocaL_EndTangent :type "Vector Structure") (LocaL_CurrentSplineMesh :type "SplineMeshComponent Object Reference"))
  (bind (_location _tangent) (`SplineComponent.GetLocationAndTangentAtSplinePoint` (`self.Spline`) (`local.LocaL_NextLoopIndex`) "Local"))
  (bind (_location_2 _tangent_2) (`SplineComponent.GetLocationAndTangentAtSplinePoint` (`self.Spline`) (`local.LocaL_CurrentLoopIndex`) "Local"))
  (set `local.LocaL_CurrentLoopIndex` LoopIndex)
  (set `local.LocaL_NextLoopIndex` (mod (+ LoopIndex 1) (`self.NumberOfSplinePoints`)))
  (set `local.LocaL_TrackElementMesh` TrackElementMesh)
  (`|ExecutionSequence`
    (:`then_0`
      (set `local.LocaL_StartLocation` _location_2)
      (set `local.LocaL_StartTangent` _tangent_2)
      (set `local.LocaL_EndLocation` _location)
      (set `local.LocaL_EndTangent` _tangent))
    (:`then_1`
      (bind _returnvalue (`AddComponent|NODE_AddSplineMeshComponent-0`))
      (set `local.LocaL_CurrentSplineMesh` _returnvalue)
      (`StaticMeshComponent.SetStaticMesh` (`local.LocaL_CurrentSplineMesh`) (`local.LocaL_TrackElementMesh`))
      (`SplineMeshComponent.SetStartAndEnd` (`local.LocaL_CurrentSplineMesh`) (`local.LocaL_StartLocation`) (`local.LocaL_StartTangent`) (`local.LocaL_EndLocation`) (`local.LocaL_EndTangent`) true))))

(fn `UserConstructionScript`
  (bind _roaddataarray (`self.RoadDataArray`))
  (`|ExecutionSequence`
    (:`then_0`
      (set `self.NumberOfSplinePoints` (`SplineComponent.GetNumberOfSplinePoints` (`self.Spline`))))
    (:`then_1`
      (`/Engine/EditorBlueprintResources/StandardMacros.CompareInt` (`KismetArrayLibrary.Array_Length` (`self.RoadDataArray`)) (`self.NumberOfSplinePoints`) :!label _label
        (:`>`
          (`KismetArrayLibrary.Array_Remove` _roaddataarray (`KismetArrayLibrary.Array_LastIndex` _roaddataarray))
          (goto _label))
        (:`<`
          (`KismetArrayLibrary.Array_Add` (`self.RoadDataArray`))
          (goto _label))))
    (:`then_2`
      (for _index (range (`self.NumberOfSplinePoints`))
        (`self.Build Track Element` _index (`self.RoadMesh`))))
    (:`then_3`)))